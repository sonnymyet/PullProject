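; Attract is an unfinished Blueprint that caches its owning Pawn, apparently as groundwork for moving it to a target position.
; On first click it records the owner's current location, sets a selected flag and prints that flag.
; The MovetoLocation event only checks the flag; the location setters are disconnected and the VInterpTo interpolation is unused, so nothing moves yet.
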(event EventBeginPlay
  (bind _aspawn (Utilities|Casting|CastToPawn (Components|GetOwner)))
  (Variables|Default|SetOwner _aspawn))

(event EventOnFirstClick
  (Variables|Default|SetCurrentPosition (Transformation|GetActorLocation (Variables|Default|GetOwner)))
  (bind _output_get (Variables|Default|SetIsSelected true))
  (Development|PrintString (Utilities|String|ToString(Boolean) _output_get)))

(event EventMovetoLocation
  (if (Variables|Default|GetIsSelected)
    _))