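; Gate is a physics-driven environment actor that the player pushes up or down with the mouse.
; A trigger volume enables player input on the gate while a CharacterBP overlaps it and disables it when the overlap ends.
; Hovering sets a flag and shows a hand cursor; left or right click then applies a large vertical force to the mesh and prints the direction.
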(event OnComponentBeginOverlap(Trigger)
  (params (OtherActor :type Actor%20Object%20Reference) (OtherComp :type Primitive%20Component%20Object%20Reference) (OtherBodyIndex :type Integer) (bFromSweep :type Boolean) (SweepResult :type Hit%20Result%20Structure%20%28by%20ref%29))
  ;[1 1 1] Proximity Trigger
  (Utilities|Casting|CastToCharacterBP OtherActor)
  (Input|EnableInput (Game|GetPlayerController 0)))

(event OnComponentEndOverlap(Trigger)
  (params (OtherActor :type Actor%20Object%20Reference) (OtherComp :type Primitive%20Component%20Object%20Reference) (OtherBodyIndex :type Integer))
  ;[1 1 1] Proximity Trigger
  (Utilities|Casting|CastToCharacterBP OtherActor)
  (Input|DisableInput (Game|GetPlayerController 0)))

(event MouseInput|EventActorBeginCursorOver
  ;[1 1 1] Mouse Over
  (Variables|Default|SetCursor%20Over true)
  (Variables|/Script/Engine.PlayerController|SetCurrentMouseCursor (Game|GetPlayerController 0) "Hand"))

(event MouseInput|EventActorEndCursorOver
  (bind _returnvalue (Game|GetPlayerController 0))
  ;[1 1 1] Mouse Over
  (Variables|Default|SetCursor%20Over false)
  (Variables|/Script/Engine.PlayerController|SetCurrentMouseCursor _returnvalue (Variables|/Script/Engine.PlayerController|GetDefaultMouseCursor _returnvalue)))

(event Input|MouseEvents|LeftMouseButton
  (params (Key :type Key%20Structure :default "AnyKey"))
  ;[1 1 1] Attract Ability
  (:Pressed
    (if (Variables|Default|GetCursor%20Over)
      (Physics|AddForce (Variables|Debug|GetStaticMeshComponent) "0, 0,50000000.000000" "None" false)
      (Development|PrintString "Up"))))

(event Input|MouseEvents|RightMouseButton
  (params (Key :type Key%20Structure :default "AnyKey"))
  ;[1 1 1] Attract Ability
  (:Pressed
    (if (Variables|Default|GetCursor%20Over)
      (Physics|AddForce (Variables|Debug|GetStaticMeshComponent) "0, 0,-50000000.000000" "None" false)
      (Development|PrintString "Down"))))

(fn ConstructionScript)