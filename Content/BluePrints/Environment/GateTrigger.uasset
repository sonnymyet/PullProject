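; Trigger actor that opens a referenced gate after a Giant enters its sphere.
; A Giant overlapping the sphere starts a short delay, after which the trigger destroys itself.
; OpenGate is bound to the actor's destroyed event at BeginPlay and sets TriggerGate on GateRef, so destruction itself is the opening signal.
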(event OnComponentBeginOverlap(Sphere)
  (params (OtherActor :type Actor%20Object%20Reference) (OtherComp :type Primitive%20Component%20Object%20Reference) (OtherBodyIndex :type Integer) (bFromSweep :type Boolean) (SweepResult :type Hit%20Result%20Structure%20%28by%20ref%29))
  (bind _asgiant (Utilities|Casting|CastToGiant OtherActor))
  (if (Utilities|IsValid _asgiant)
    (Utilities|FlowControl|Delay 3.0)
    (Actor|DestroyActor)))

(event Custom|OpenGate
  (bind _gateref (Variables|Default|GetGateRef))
  (if (Utilities|IsValid _gateref)
    (Variables|/Game/BluePrints/Environment/Gate.Gate_C|SetTriggerGate _gateref true)))

(event EventBeginPlay
  (EventDispatchers|BindEventtoOnDestroyed (delegate Custom|OpenGate)))

(fn ConstructionScript)