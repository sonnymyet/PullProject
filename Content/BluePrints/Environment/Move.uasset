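; Environment actor Blueprint that relays mouse interaction to its AttractibleComponent, apparently so the object can be moved.
; Cursor over, cursor end and click events forward to the component's custom handlers.
; Clicking also enables player input on the actor, so later left mouse presses call the component's UpdateNewPosition.
; The movement logic lives in the component, and this graph never disables the input again.
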(event OnClicked(CapsuleComponent)
  (params (TouchedComponent :type Primitive%20Component%20Object%20Reference)))

(event MouseInput|EventActorBeginCursorOver
  ;[1 1 1] Custom Mouse Over
  (Default|CustomActorBeginCursorOver (Variables|Default|GetAttractibleComponent)))

(event MouseInput|EventActorEndCursorOver
  ;[1 1 1] Custom Mouse Over
  (Default|CustomActorEndCursorOver (Variables|Default|GetAttractibleComponent)))

(event MouseInput|EventActorOnClicked
  (Default|CustomonClick (Variables|Default|GetAttractibleComponent))
  (Input|EnableInput (Game|GetPlayerController 0)))

(event Input|MouseEvents|LeftMouseButton
  (params (Key :type Key%20Structure :default "AnyKey"))
  (:Pressed
    (Default|UpdateNewPosition (Variables|Default|GetAttractibleComponent))))

(fn ConstructionScript)