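; Actor component that lets its owning actor be picked up with a click and moved with the mouse cursor.
; Externally triggered events switch the cursor to a hand on hover, toggle the clicked state, and project the mouse 1000 units into the world as the target.
; While active, Tick moves the owner there through a Lerp with alpha 1, so it snaps.
; The timer-driven Move To Position route is disconnected, and debug prints remain.
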(event Custom|Custom%20On%20Click
  (if (Variables|Default|GetIsClicked)
    (Variables|Default|SetIsClicked false)
    (else
      (Variables|Default|SetIsClicked true)))
  (Variables|Default|SetCurrent%20Position (Transformation|GetActorLocation (Components|GetOwner))))

(event Custom|UpdateNewPosition
  (bind _returnvalue (Game|GetPlayerController 0))
  (bind (_worldlocation _worlddirection) (Game|Player|ConvertMouseLocationToWorldSpace _returnvalue))
  (if (Variables|Default|GetIsClicked)
    (bind _output_get (Variables|Default|SetTarget%20Position (+ _worldlocation (* _worlddirection 1e+03))))
    (Variables|Default|SetPositionUpdated true)
    (Development|PrintString (Utilities|String|ToString(Vector) _output_get))
    (else
      (Variables|Default|SetPositionUpdated false))))

(event Custom|Move%20Actor)

(event Custom|CustomActorBeginCursorOver
  ;[1 1 1] Mouse Over
  (Variables|Default|SetCursor%20Over true)
  (Variables|/Script/Engine.PlayerController|SetCurrentMouseCursor (Game|GetPlayerController 0) "Hand"))

(event Custom|CustomActorEndCursorOver
  (bind _returnvalue (Game|GetPlayerController 0))
  ;[1 1 1] Mouse Over
  (Variables|Default|SetCursor%20Over false)
  (Variables|/Script/Engine.PlayerController|SetCurrentMouseCursor _returnvalue (Variables|/Script/Engine.PlayerController|GetDefaultMouseCursor _returnvalue)))

(event EventBeginPlay
  (Variables|Default|SetAttached%20Actor (Components|GetOwner)))

(event EventTick
  (params (DeltaSeconds :type Float%20%28single-precision%29))
  (if (and (Variables|Default|GetIsClicked) (Variables|Default|GetPositionUpdated))
    (bind _returnvalue (Transformation|SetActorLocation (Variables|Default|GetAttached%20Actor) (Math|Vector|Lerp(Vector) (Variables|Default|GetCurrent%20Position) (Variables|Default|GetTarget%20Position) 1.0) false false))))

(fn MovetoPosition
  (Transformation|SetActorLocation (Components|GetOwner) (Math|Vector|Lerp(Vector) (Variables|Default|GetCurrent%20Position) (Variables|Default|GetTarget%20Position) 1.0) false false)
  (Development|PrintString "Move Function"))