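; EnemyAI is an enemy Blueprint that wanders at random until it sees the player character, then moves toward it.
; On Tick, it starts an AIMoveTo to a random reachable point nearby, with OnChase blocking new wander moves until the current one succeeds or fails.
; PawnSensing sets TargetInRange for any seen pawn, permanently stopping new wander moves, and issues AIMoveTo toward that pawn if it casts to CharacterBP.
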(event OnSeePawn(PawnSensing)
  (params (Pawn :type Pawn%20Object%20Reference))
  (Variables|Default|SetTarget%20In%20Range true)
  (bind _ascharacter_bp (Utilities|Casting|CastToCharacterBP Pawn))
  (AI|AIMoveTo self "0, 0, 0" _ascharacter_bp 1e+01 false))

(event EventBeginPlay)

(event EventActorBeginOverlap
  (params (OtherActor :type Actor%20Object%20Reference)))

(event EventTick
  (params (DeltaSeconds :type Float%20%28single-precision%29))
  (if (not (Variables|Default|GetTarget%20In%20Range))
    (if (not (Variables|Default|GetOn%20Chase))
      (AI|AIMoveTo self (AI|Navigation|GetRandomReachablePointinRadius (Transformation|GetActorLocation) 1e+03) 0 5.0 false
        (:then
          (Variables|Default|SetOn%20Chase true))
        (:OnSuccess
          (Variables|Default|SetOn%20Chase false :!label _label))
        (:OnFail
          (goto _label))))))

(fn ConstructionScript)