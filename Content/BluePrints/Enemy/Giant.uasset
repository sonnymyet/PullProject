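; Giant is an enemy Blueprint that chases the player character once it has seen it.
; PawnSensing stores a seen CharacterBP and sets TargetInRange, which nothing here resets.
; While that flag is true, Tick issues AI MoveTo toward the character every frame.
; OnChase tracks the move but is never read, debug prints show both flags, and a random-wander move is left unconnected.
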(event OnSeePawn(PawnSensing)
  (params (Pawn :type Pawn%20Object%20Reference))
  (bind _ascharacter_bp (Utilities|Casting|CastToCharacterBP Pawn))
  (bind _output_get (Variables|Default|SetTargetInRange true))
  (Development|PrintString (Utilities|String|ToString(Boolean) _output_get)))

(event EventTick
  (params (DeltaSeconds :type Float%20%28single-precision%29))
  (if (Variables|Default|GetTargetInRange)
    (AI|AIMoveTo self "0, 0, 0" (stale OnSeePawn(PawnSensing) _ascharacter_bp) 1e+01 false
      (:then
        (Variables|Default|SetOnChase true))
      (:OnSuccess
        (bind _output_get (Variables|Default|SetOnChase false :!label _label))
        (Development|PrintString (Utilities|String|ToString(Boolean) _output_get)))
      (:OnFail
        (goto _label)))))

(fn ConstructionScript)