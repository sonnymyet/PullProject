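; Spider enemy Blueprint that wanders at random and chases the player character when it sees one.
; On Tick, with no target and no move in progress, it moves to a random reachable point nearby.
; PawnSensing sighting a CharacterBP starts an AI move toward it, and the target clears when that move succeeds or fails.
; Trigger overlap with instanced foliage clears the OnChase movement flag, letting an untargeted spider pick a new point.
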(event OnComponentBeginOverlap(Trigger)
  (params (OtherActor :type Actor%20Object%20Reference) (OtherComp :type Primitive%20Component%20Object%20Reference) (OtherBodyIndex :type Integer) (bFromSweep :type Boolean) (SweepResult :type Hit%20Result%20Structure%20%28by%20ref%29))
  (Utilities|Casting|CastToInstancedFoliageActor OtherActor)
  (Variables|Default|SetOn%20Chase false))

(event OnSeePawn(PawnSensing)
  (params (Pawn :type Pawn%20Object%20Reference))
  (bind _ascharacter_bp (Utilities|Casting|CastToCharacterBP Pawn))
  (Variables|Default|SetTarget%20In%20Range true)
  (AI|AIMoveTo self "0, 0, 0" _ascharacter_bp 1e+01 false
    (:then
      (Variables|Default|SetOn%20Chase true))
    (:OnSuccess
      (Variables|Default|SetOn%20Chase false :!label _label)
      (Variables|Default|SetTarget%20In%20Range false))
    (:OnFail
      (goto _label))))

(event EventTick
  (params (DeltaSeconds :type Float%20%28single-precision%29))
  (if (not (Variables|Default|GetTarget%20In%20Range))
    (if (not (Variables|Default|GetOn%20Chase))
      (AI|AIMoveTo self (AI|Navigation|GetRandomReachablePointinRadius (Transformation|GetActorLocation) 1e+03) 0 5.0 false
        (:then
          (Variables|Default|SetOn%20Chase true))
        (:OnSuccess
          (Variables|Default|SetOn%20Chase false :!label _label))
        (:OnFail
          (goto _label))))))

(fn ConstructionScript)