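; PullGameMode is a game mode that populates the level with enemy spiders and gravity orbs and handles player respawning.
; On BeginPlay it starts a looping SpawnEnemy timer on every EnemySpawner, using EnemiesPerSecond as the interval.
; It also spawns an enlarged AbilityRune orb at every TargetPoint in the level.
; RespawnPlayer waits briefly, spawns a new CharacterBP at PlayerSpawnTransform and has the first player controller possess it.
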(event Custom|Respawn%20Player
  ;[1 1 1] Spawn Player
  (Utilities|FlowControl|Delay 1.5)
  (bind _returnvalue (Game|SpawnActorfromClass "/Game/BluePrints/Character/CharacterBP.CharacterBP_C" (Variables|Default|GetPlayerSpawnTransform) "Undefined" 0 0))
  (Pawn|Possess (Game|GetPlayerController 0) _returnvalue))

(event Custom|SpawnOrbs
  ;[1 1 1] Spawn Gravity Orbs
  (bind _outactors (Actor|GetAllActorsOfClass "/Script/Engine.TargetPoint"))
  (for _array_element _outactors
    (Game|SpawnActorfromClass "/Game/BluePrints/Collectibles/AbilityRune.AbilityRune_C" (Math|Transform|MakeTransform (Transformation|GetActorLocation _array_element) "0, 0, 0" "5.000000,5.000000,5.000000") "Undefined" 0 0)))

(event Custom|SpawnSpiders
  ;[1 1 1] Spawn Spiders
  (bind _outactors (Actor|GetAllActorsOfClass "/Game/BluePrints/Enemy/EnemySpawner.EnemySpawner_C"))
  (for _array_element _outactors
    (bind _output_get (Variables|Default|SetEnemySpawner _array_element))
    (Utilities|Time|SetTimerbyFunctionName _output_get "SpawnEnemy" (Variables|Default|GetEnemiesPerSecond) true)))

(event EventBeginPlay
  (Utilities|FlowControl|Sequence
    (:then_0
      (CallFunction|SpawnSpiders))
    (:then_1
      (CallFunction|SpawnOrbs))))

(fn ConstructionScript)