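; Actor component that lifts its owner's physics body when clicked and gives hand-cursor feedback on mouse-over.
; BeginPlay enables physics simulation on the owner's first primitive component.
; When the OnClick flag is set, Tick disables gravity, raises the body 10 units without sweeping and clears the flag.
; Cursor-over events track hover state and swap the cursor; nothing here sets OnClick or restores gravity.
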(event Custom|ReceiveActorBeginCursorOver_Copy
  ;[1 1 1] Mouse Over
  (Variables|Default|SetCursor%20Over true)
  (Variables|/Script/Engine.PlayerController|SetCurrentMouseCursor (Game|GetPlayerController 0) "Hand"))

(event Custom|ReceiveActorEndCursorOver_Copy
  (bind _returnvalue (Game|GetPlayerController 0))
  ;[1 1 1] Mouse Over
  (Variables|Default|SetCursor%20Over false)
  (Variables|/Script/Engine.PlayerController|SetCurrentMouseCursor _returnvalue (Variables|/Script/Engine.PlayerController|GetDefaultMouseCursor _returnvalue)))

(event EventBeginPlay
  (bind _output_get (Variables|Default|SetPrimitiveComponent (Utilities|Array|Get(acopy) (Actor|GetComponentsByClass (Components|GetOwner) "/Script/Engine.PrimitiveComponent"))))
  (Physics|SetSimulatePhysics _output_get true))

(event EventTick
  (params (DeltaSeconds :type Float%20%28single-precision%29))
  (bind _returnvalue (Transformation|GetWorldLocation))
  (bind _primitivecomponent (Variables|Default|GetPrimitiveComponent))
  (bind (_x _y _z) (Math|Vector|BreakVector _returnvalue))
  (if (Variables|Default|GetOnClick)
    (Physics|SetEnableGravity _primitivecomponent false)
    (Transformation|SetWorldLocation _primitivecomponent (Math|Vector|MakeVector _x _y (+ _z 1e+01)) false false)
    (Variables|Default|SetOnClick false)))