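; HoverComponent2 is an actor component that lifts its owner upward when triggered.
; On BeginPlay it caches the owner's first primitive component and enables physics simulation on it.
; Tick polls an OnClick flag, which this graph only clears, then disables gravity and calls MoveComponentTo toward 100 units higher.
; The relative-location target is built from the component's world location, and gravity is never re-enabled here.
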(event EventBeginPlay
  (bind _output_get (Variables|Default|SetStatic%20Mesh%20Actor (Utilities|Array|Get(acopy) (Actor|GetComponentsByClass (Components|GetOwner) "/Script/Engine.PrimitiveComponent"))))
  (Physics|SetSimulatePhysics _output_get true))

(event EventTick
  (params (DeltaSeconds :type Float%20%28single-precision%29))
  (bind _static_mesh_actor (Variables|Default|GetStatic%20Mesh%20Actor))
  (bind _returnvalue (Transformation|GetWorldLocation _static_mesh_actor))
  (bind (_x _y _z) (Math|Vector|BreakVector _returnvalue))
  (if (Variables|Default|GetOnClick)
    (Physics|SetEnableGravity _static_mesh_actor false)
    (Components|MoveComponentTo _static_mesh_actor (Math|Vector|MakeVector _x _y (+ _z 1e+02)) "0, 0, 0" false false 0.2)
    (Variables|Default|SetOnClick false)))