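; Component that lets the player click-select its owning pawn and pull it to a target position.
; Hover and click events update the cursor and selection state, with killable pawns never selected, while SetTarget stores the destination.
; MovetoLocation loops through a Gate and short Delay, interpolating the pawn until within collision range.
; On arrival it destroys the first overlapping Spider and resets selection, target and cursor.
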(event Custom|CustomActorBeginCursorOver
  ;[1 1 1] Mouse Over
  (Variables|/Script/Engine.PlayerController|SetCurrentMouseCursor (Game|GetPlayerController 0) "Hand"))

(event Custom|CustomActorEndCursorOver
  (bind _returnvalue (Game|GetPlayerController 0))
  ;[1 1 1] Mouse Over
  (if (Variables|Default|GetIsSelected)
    (Variables|/Script/Engine.PlayerController|SetbEnableMouseOverEvents _returnvalue false)
    (else
      (Variables|/Script/Engine.PlayerController|SetCurrentMouseCursor _returnvalue (Variables|/Script/Engine.PlayerController|GetDefaultMouseCursor _returnvalue))
      (Variables|/Script/Engine.PlayerController|SetbEnableMouseOverEvents _returnvalue true))))

(event EventBeginPlay
  (bind _aspawn (Utilities|Casting|CastToPawn (Components|GetOwner)))
  (bind _output_get (Variables|Default|SetOwner _aspawn))
  (EventDispatchers|BindEventtoOnBeginCursorOver _output_get (delegate Custom|CustomActorBeginCursorOver))
  (EventDispatchers|BindEventtoOnEndCursorOver _output_get (delegate Custom|CustomActorEndCursorOver)))

(event EventOnFirstClick
  ;[1 1 1] First Click Interaction
  (if (Variables|Default|GetIsKillable)
    (Variables|Default|SetIsSelected false)
    (else
      (Variables|Default|SetCurrentPosition (Transformation|GetActorLocation (Variables|Default|GetOwner)))
      (Variables|Default|SetIsSelected true)
      (Variables|/Script/Engine.PlayerController|SetCurrentMouseCursor (Game|GetPlayerController 0) "GrabHandClosed"))))

(event EventMovetoLocation
  (bind _returnvalue (Game|GetPlayerController 0))
  (bind _owner (Variables|Default|GetOwner))
  (bind _targetposition (Variables|Default|GetTargetPosition))
  (bind _overlappingactors (Collision|GetOverlappingActors _owner "/Game/BluePrints/Enemy/Spider.Spider_C" :!class /Script/Engine.Actor))
  (bind _item (Utilities|Array|Get(acopy) _overlappingactors))
  ;[1 1 1] Move To Location
  (if (and (Variables|Default|GetIsSelected) (Variables|Default|GetTarget))
    (Variables|/Script/Engine.PlayerController|SetCurrentMouseCursor (Game|GetPlayerController 0) "Hand")
    (Utilities|FlowControl|Sequence
      (:then_0
        (goto _label_2 Open))
      (:then_1
        (Transformation|SetActorLocation (Variables|Default|GetOwner) (Math|Interpolation|VInterpTo (Variables|Default|GetCurrentPosition) _targetposition (Utilities|Time|GetWorldDeltaSeconds) 4.5) false false :!label _label)
        (Utilities|FlowControl|Delay 0.01)
        (Utilities|FlowControl|Sequence
          (:then_0
            (Utilities|FlowControl|Gate true :!label _label_2
              (:Exit
                (goto _label))))
          (:then_1
            (if (Math|Vector|Equal(Vector) (Variables|Default|GetCurrentPosition) _targetposition (Variables|Default|GetCollisionRange))
              (Utilities|FlowControl|Sequence
                (:then_0
                  (goto _label_2 Close))
                (:then_1
                  (if (Utilities|IsValid _item)
                    (Actor|DestroyActor _item)))
                (:then_2
                  (Variables|/Script/Engine.PlayerController|SetCurrentMouseCursor _returnvalue "CardinalCross")
                  (Variables|/Script/Engine.PlayerController|SetbEnableMouseOverEvents _returnvalue true))
                (:then_3
                  (Variables|Default|SetIsSelected false)
                  (Variables|Default|SetTarget false)))
              (else
                (Variables|Default|SetCurrentPosition (Transformation|GetActorLocation _owner))))))))))

(fn SetTarget
  (params (TargetPosition :type Vector))
  (Variables|Default|SetTargetPosition TargetPosition)
  (Variables|Default|SetTarget true))

(fn NewFunction0)