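; GravityOrb is a collectible that adds a gem to CharacterBP and destroys its AbilityRune component when the character overlaps its Trigger.
; The actor itself remains, toggling input and a PlayerInRange flag on overlap, so every re-entry adds another gem.
; Hovering sets a CursorOver flag and shows a hand cursor.
; Up and down force logic for the rune, under an "Attract Ability" comment, is disconnected and never runs.
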(event OnComponentBeginOverlap(Trigger)
  (params (OtherActor :type Actor%20Object%20Reference) (OtherComp :type Primitive%20Component%20Object%20Reference) (OtherBodyIndex :type Integer) (bFromSweep :type Boolean) (SweepResult :type Hit%20Result%20Structure%20%28by%20ref%29))
  ;[1 1 1] Proximity Trigger
  (bind _ascharacter_bp (Utilities|Casting|CastToCharacterBP OtherActor))
  (Input|EnableInput (Game|GetPlayerController 0))
  (Variables|Default|SetPlayer%20In%20Range true)
  (Variables|/Game/BluePrints/Character/CharacterBP.CharacterBP_C|SetGems _ascharacter_bp (+ (Variables|/Game/BluePrints/Character/CharacterBP.CharacterBP_C|GetGems _ascharacter_bp) 1))
  (Components|DestroyComponent (Variables|Default|GetAbilityRune)))

(event OnComponentEndOverlap(Trigger)
  (params (OtherActor :type Actor%20Object%20Reference) (OtherComp :type Primitive%20Component%20Object%20Reference) (OtherBodyIndex :type Integer))
  ;[1 1 1] Proximity Trigger
  (Utilities|Casting|CastToCharacterBP OtherActor)
  (Input|DisableInput (Game|GetPlayerController 0))
  (Variables|Default|SetPlayer%20In%20Range false))

(event MouseInput|EventActorBeginCursorOver
  ;[1 1 1] Mouse Over
  (Variables|Default|SetCursorOver true)
  (Variables|/Script/Engine.PlayerController|SetCurrentMouseCursor (Game|GetPlayerController 0) "Hand"))

(event MouseInput|EventActorEndCursorOver
  (bind _returnvalue (Game|GetPlayerController 0))
  ;[1 1 1] Mouse Over
  (Variables|Default|SetCursorOver false)
  (Variables|/Script/Engine.PlayerController|SetCurrentMouseCursor _returnvalue (Variables|/Script/Engine.PlayerController|GetDefaultMouseCursor _returnvalue)))

(event EventBeginPlay)

(event Input|MouseEvents|LeftMouseButton
  (params (Key :type Key%20Structure :default "AnyKey"))
  ;[1 1 1] Attract Ability
)

(event Input|MouseEvents|RightMouseButton
  (params (Key :type Key%20Structure :default "AnyKey"))
  ;[1 1 1] Attract Ability
)

(fn ConstructionScript)